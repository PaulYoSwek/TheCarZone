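; Vehicle weaponry component for cars, largely disconnected: its SetCurrentWeapon, BeginPlay and UseWeapon entry points are empty.
; Unwired logic spawns a weapon at its class-default socket on the CarBase body, attaches it to this component and defaults to boxing gloves.
; ReleaseWeapon still forwards to the active weapon.
; UpdatePhysicsConstraint, called only from that unwired logic, constrains BP_Car's body to the component.
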(event `SetCurrentWeapon`
  (params (NewParam :type "/Game/GoodFolderStructure/Assets/Weapons/Base/BP_WeaponBase Class Reference")))

(event `self.ReceiveBeginPlay`)

(fn `ReleaseWeapon`
  (`/Game/GoodFolderStructure/Assets/Weapons/Base/BP_WeaponBase.ReleaseWeapon` (`self.ActiveWeapon`)))

(fn `UpdatePhysicsConstraint`
  (bind _asbp_car (cast `/Game/GoodFolderStructure/Blueprints/Vehicle/BP_Car` (`self.GetOwner`))
    (:`then`
      (`PhysicsConstraintComponent.SetConstrainedComponents` (`/Game/GoodFolderStructure/Blueprints/Vehicle/BP_Car.PhysicsConstraint_Weapon` _asbp_car) (`VehicleBase.Body` _asbp_car) "None" self "None"))
    (:`CastFailed`
      (`KismetSystemLibrary.PrintString` "PAS OP PIKKIE: BP_VehicleWeaponryComponent PhysicsConstraint cast failed! das nie de bedoeling :(" true true (struct :`R` 1.0 :`G` 0.028356 :`A` 1.0) 100.0))))

(fn `UseWeapon`)