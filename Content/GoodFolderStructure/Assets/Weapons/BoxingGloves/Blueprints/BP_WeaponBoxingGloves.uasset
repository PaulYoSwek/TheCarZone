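; Boxing glove weapon that throws alternating spring-loaded punches, pushing physics objects it hits.
; ExecuteWeapon ignores calls while executing, otherwise toggles the active glove and spring and starts the BoxingMotion timeline.
; The timeline scales the spring and sweeps it and the glove along local X, ending the forward phase near peak extension.
; Hit events on the active glove apply force against the impact normal only during that forward phase.
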(event `BoxingMotionEvent`
  (bind _currentstrikingspring (`self.CurrentStrikingSpring`))
  (bind (_direction _springscale) (`Timeline|BoxingMotion` :!via `PlayFromStart`)
    (:`Update`
      (`SceneComponent.SetRelativeScale3D` _currentstrikingspring (`KismetMathLibrary.MakeVector` _springscale))
      (bind _returnvalue (* (`self.UnitsMovedPer1Scale`) _springscale))
      (`SceneComponent.K2_SetRelativeLocation` _currentstrikingspring (`KismetMathLibrary.MakeVector` _returnvalue) true false)
      (`SceneComponent.K2_SetRelativeLocation` (`self.CurrentStrikingGlove`) (`KismetMathLibrary.MakeVector` _returnvalue) true false)
      (if (>= _springscale 1.49)
        (set `self.bGloveGoingForward` false)))
    (:`Finished`
      (set `self.bIsExecuting` false))))

(event `self.Glove1.OnComponentHit`
  (params (HitComponent :type "PrimitiveComponent Object Reference") (OtherActor :type "Actor Object Reference") (OtherComp :type "PrimitiveComponent Object Reference") (NormalImpulse :type "Vector Structure") (Hit :type "HitResult Structure (by ref)"))
  (bind (_bblockinghit _binitialoverlap _time _distance _location _impactpoint _normal _impactnormal) (`GameplayStatics.BreakHitResult` Hit))
  (if (and (`self.bGloveGoingForward`) (`self.bGlove1GetsToPunch`))
    (`PrimitiveComponent.AddForceAtLocation` OtherComp (* (* _impactnormal (-1.0 -1.0 -1.0)) (`self.PunchForce`)) _impactpoint "None")))

(event `self.Glove2.OnComponentHit`
  (params (HitComponent :type "PrimitiveComponent Object Reference") (OtherActor :type "Actor Object Reference") (OtherComp :type "PrimitiveComponent Object Reference") (NormalImpulse :type "Vector Structure") (Hit :type "HitResult Structure (by ref)"))
  (bind (_bblockinghit _binitialoverlap _time _distance _location _impactpoint _normal _impactnormal) (`GameplayStatics.BreakHitResult` Hit))
  (if (and (`self.bGloveGoingForward`) (not (`self.bGlove1GetsToPunch`)))
    (`PrimitiveComponent.AddForceAtLocation` OtherComp (* (* _impactnormal (-1.0 -1.0 -1.0)) (`self.PunchForce`)) _impactpoint "None")))

(fn `ExecuteWeapon`
  (if (not (`self.bIsExecuting`))
    (`parent.ExecuteWeapon`)
    (bind _output_get (set `self.bGlove1GetsToPunch` (not (`self.bGlove1GetsToPunch`))))
    (set `self.bGloveGoingForward` true)
    (`self.BoxingMotionEvent`)
    (if _output_get
      (set `self.CurrentStrikingSpring` (`self.Spring1`))
      (set `self.CurrentStrikingGlove` (`self.Glove1`))
      (else
        (set `self.CurrentStrikingSpring` (`self.Spring2`))
        (set `self.CurrentStrikingGlove` (`self.Glove2`))))))

(fn `UserConstructionScript`
  (`parent.UserConstructionScript`))