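; Test actor that spawns a row of numbered text labels in the level when play begins.
; BeginPlay loops from zero through MaxCount, spawning a TextRenderActor at each step, offset 100 units further along world Y from the spawner's location.
; Each label shows its index, doubled in scale, centered both ways and tinted with the TextColor variable.
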(event `self.ReceiveBeginPlay`
  (bind _returnvalue_location (`KismetMathLibrary.BreakTransform` (`self.GetTransform`)))
  (for _index (range (+ (`self.MaxCount`) 1))
    (`|ExecutionSequence`
      (:`then_0`
        (bind _returnvalue (`|SpawnActorFromClass` "/Script/Engine.TextRenderActor" (`KismetMathLibrary.MakeTransform` (`KismetMathLibrary.MakeVector` (.x _returnvalue_location) (+ (.y _returnvalue_location) (* _index 100)) (.z _returnvalue_location))) "AlwaysSpawn" "OverrideRootScale" null null))
        (`TextRenderComponent.K2_SetText` (`TextRenderActor.TextRender` _returnvalue) (`KismetTextLibrary.Conv_IntToText` _index))
        (`TextRenderComponent.SetYScale` (`TextRenderActor.TextRender` _returnvalue) 2.0)
        (`TextRenderComponent.SetXScale` (`TextRenderActor.TextRender` _returnvalue) 2.0)
        (`TextRenderComponent.SetTextRenderColor` (`TextRenderActor.TextRender` _returnvalue) (`self.TextColor`))
        (`TextRenderComponent.SetHorizontalAlignment` (`TextRenderActor.TextRender` _returnvalue) "EHTA_Center")
        (`TextRenderComponent.SetVerticalAlignment` (`TextRenderActor.TextRender` _returnvalue) "EVRTA_TextCenter")))))

(fn `UserConstructionScript`)