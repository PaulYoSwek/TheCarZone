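; BP_Car is a player-driven physics car with boost, a charged jump and a weapon component.
; When rear suspension has contact, it drives the body with acceleration-based force from a speed curve plus boost, and speed-scaled yaw torque that inverts in reverse.
; Front wheels turn visually within limits and recenter, while linear damping switches between ground and air.
; Holding Space presses the body down on a timeline, and releasing launches it upward.
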(event `InputAction|UseWeapon1`
  (params (Key :type "Key Structure"))
  (:`Pressed`
    (`/Game/GoodFolderStructure/Assets/Weapons/Base/BP_VehicleWeaponryComponent.UseWeapon` (`self.BP_VehicleWeaponryComponent`))))

(event `Steer`
  (params (SteerDirection :type "Float (double-precision)"))
  (set `self.SteerDirection` SteerDirection)
  (`SceneComponent.K2_SetRelativeRotation` (`self.Wheel_FR`) (`KismetMathLibrary.MakeRotator` 0.0 0.0 (`KismetMathLibrary.ClampAngle` (`self.CalculateWheelZRotation` (`self.Wheel_FR`) (`self.SteerDirection`)) -60.0 60.0)) false true)
  (`SceneComponent.K2_SetRelativeRotation` (`self.Wheel_FL`) (`KismetMathLibrary.MakeRotator` 0.0 0.0 (`KismetMathLibrary.ClampAngle` (`self.CalculateWheelZRotation` (`self.Wheel_FL`) (`self.SteerDirection`)) -60.0 60.0)) false true))

(event `InputAxis|MoveRight`
  (params (AxisValue :type "Float (single-precision)"))
  (`self.Steer` AxisValue))

(event `InputAxisKey|MouseX`
  (params (AxisValue :type "Float (single-precision)"))
  (bind (_returnvalue_roll _returnvalue_pitch _returnvalue_yaw) (`KismetMathLibrary.BreakRotator` (`self.GetControlRotation`)))
  (`self.AddControllerYawInput` AxisValue)
  (`Controller.SetControlRotation` (`MyBlueprintUtilities.GetLocalPlayerController`) (`KismetMathLibrary.MakeRotator` 0.0 _returnvalue_pitch _returnvalue_yaw)))

(event `InputAxisKey|MouseY`
  (params (AxisValue :type "Float (single-precision)"))
  (`self.AddControllerPitchInput` (* -1 AxisValue)))

(event `self.ReceiveTick`
  (params (DeltaSeconds :type "Float (single-precision)"))
  (`self.UpdateLinearDamping`))

(event `InputAxis|MoveForward`
  (params (AxisValue :type "Float (single-precision)"))
  (`self.CalculateSpeed` AxisValue)
  (`self.MoveForward` AxisValue))

(event `MoveForward`
  (params (Direction :type "Float (double-precision)"))
  (bind _steerdirection (`self.SteerDirection`))
  (bind (_relativerotation_roll _relativerotation_pitch _relativerotation_yaw) (`KismetMathLibrary.BreakRotator` (`SceneComponent.RelativeRotation` (`self.Wheel_FL`))))
  (bind (_relativerotation_roll_2 _relativerotation_pitch_2 _relativerotation_yaw_2) (`KismetMathLibrary.BreakRotator` (`SceneComponent.RelativeRotation` (`self.Wheel_FR`))))
  (set `self.Direction` Direction)
  (if (`self.IsGrounded`)
    (`PrimitiveComponent.AddForce` (`self.Body`) (* (* (`SceneComponent.GetForwardVector` (`self.Body`)) (`self.GetFinalSpeed`)) (`self.Direction`)) "None" true)
    (`PrimitiveComponent.AddTorqueInRadians` (`self.Body`) (`KismetMathLibrary.MakeVector` 0.0 0.0 (`KismetMathLibrary.Lerp` 0.0 (* (`KismetMathLibrary.SelectFloat` _steerdirection (* _steerdirection -1.0) (>= (`KismetMathLibrary.Dot_VectorVector` (`KismetMathLibrary.Normal` (`self.GetActorForwardVector`)) (`KismetMathLibrary.Normal` (`SceneComponent.GetComponentVelocity` (`self.Body`)))) 0.0)) (`self.TurnSpeed`)) (`KismetMathLibrary.MultiplyMultiply_FloatFloat` (`KismetMathLibrary.FClamp` (`KismetMathLibrary.NormalizeToRange` (`KismetMathLibrary.VSize` (`self.GetVelocity`)) 0.0 500.0)) 3.0))) "None" true)
    (if (== (`self.SteerDirection`) 0.0)
      (`SceneComponent.K2_SetRelativeRotation` (`self.Wheel_FR`) (`KismetMathLibrary.MakeRotator` 0.0 0.0 (`KismetMathLibrary.FInterpTo` _relativerotation_yaw_2 0.0 (`GameplayStatics.GetWorldDeltaSeconds`) 20.0)) false false)
      (`SceneComponent.K2_SetRelativeRotation` (`self.Wheel_FL`) (`KismetMathLibrary.MakeRotator` 0.0 0.0 (`KismetMathLibrary.FInterpTo` _relativerotation_yaw 0.0 (`GameplayStatics.GetWorldDeltaSeconds`) 20.0)) false false))))

(event `Boost`
  (params (InBoost :type "Float (double-precision)"))
  (bind (_direction _booster) (`Timeline|BoostTimeLine` :!via `PlayFromStart` :!label _label)
    (:`Update`
      (set `self.CurrentBoost` (+ (`self.CurrentBoost`) (* _booster InBoost))))))

(event `CancelBoost`
  (set `self.CurrentBoost` 0.0)
  (goto _label :!via `Stop`))

(event `Key|SpaceBar`
  (params (Key :type "Key Structure"))
  (:`Pressed`
    (`self.ChargeJump`))
  (:`Released`
    (`self.ReleaseJump`)))

(event `ChargeJump`
  (set `self.ChargingJump` true)
  (bind (_direction _chargejumptrack) (`Timeline|ChargeJumpTimeLine` :!via `PlayFromStart` :!label _label_2)
    (:`Update`
      (if (`self.ChargingJump`)
        (set `self.ChargedJumpPower` (* _chargejumptrack (`self.MaxChargeJumpPower`)))
        (`PrimitiveComponent.AddForce` (`self.Body`) (* (`KismetMathLibrary.NegateVector` (`SceneComponent.GetUpVector` (`self.Body`))) (`self.ChargedJumpPower`)) "None" true)
        (else
          (goto _label_2 :!via `Stop`))))))

(event `ReleaseJump`
  (set `self.ChargingJump` false)
  (`PrimitiveComponent.AddForce` (`self.Body`) (* (`SceneComponent.GetUpVector` (`self.Body`)) (* (`self.ChargedJumpPower`) 100.0)) "None" true))

(fn `CalculateSpeed`
  (params (InDirection :type "Float (double-precision)"))
  (if (not (== InDirection 0.0))
    (set `self.SpeedAccelTime` (`KismetMathLibrary.FClamp` (+ (`self.SpeedAccelTime`) (`GameplayStatics.GetWorldDeltaSeconds`)) 0.0 (`.MaxTime` (`CurveBase.GetTimeRange` (`self.SpeedAccellCurve`)))))
    (set `self.CurrentSpeed` (`CurveFloat.GetFloatValue` (`self.SpeedAccellCurve`) (`self.SpeedAccelTime`)))
    (else
      (set `self.SpeedAccelTime` (`KismetMathLibrary.FClamp` (- (`self.SpeedAccelTime`) (`GameplayStatics.GetWorldDeltaSeconds`)) 0.0 (`.MaxTime` (`CurveBase.GetTimeRange` (`self.SpeedAccellCurve`)))))
      (set `self.CurrentSpeed` (`CurveFloat.GetFloatValue` (`self.SpeedAccellCurve`) (`self.SpeedAccelTime`))))))

(fn `IsGrounded`
  (returns (IsGrounded :type Boolean))
  (return (or (`/Game/GoodFolderStructure/Blueprints/Vehicle/Suspension.InContact` (`self.Suspension_RR`)) (`/Game/GoodFolderStructure/Blueprints/Vehicle/Suspension.InContact` (`self.Suspension_RL`)))))

(fn `UpdateLinearDamping`
  (`PrimitiveComponent.SetLinearDamping` (`self.Body`) (select `bool` (`self.IsGrounded`) :`false` (`self.InAirLinearDamp`) :`true` (`self.DefaulLinearDamp`) :!type "Float (single-precision)")))

(fn `UserConstructionScript`)