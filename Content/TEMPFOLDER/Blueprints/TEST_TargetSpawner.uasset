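; Test spawner actor that places a single TEST_Target at a random point inside its Box component when play begins.
; Each axis is picked independently between the box's world location minus and plus its scaled extent, so box rotation is not taken into account.
; The target spawns at five times scale, and the construction script is empty.
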(event `self.ReceiveBeginPlay`
  (bind _box (`self.Box`))
  (bind (_returnvalue_x _returnvalue_y _returnvalue_z) (`KismetMathLibrary.BreakVector` (`SceneComponent.K2_GetComponentLocation` _box)))
  (bind (_returnvalue_x_2 _returnvalue_y_2 _returnvalue_z_2) (`KismetMathLibrary.BreakVector` (`BoxComponent.GetScaledBoxExtent` _box)))
  (`|SpawnActorFromClass` "/Game/TEMPFOLDER/Blueprints/TEST_Target.TEST_Target_C" (`KismetMathLibrary.MakeTransform` (`KismetMathLibrary.MakeVector` (`KismetMathLibrary.RandomFloatInRange` (- _returnvalue_x _returnvalue_x_2) (+ _returnvalue_x _returnvalue_x_2)) (`KismetMathLibrary.RandomFloatInRange` (- _returnvalue_y _returnvalue_y_2) (+ _returnvalue_y _returnvalue_y_2)) (`KismetMathLibrary.RandomFloatInRange` (- _returnvalue_z _returnvalue_z_2) (+ _returnvalue_z _returnvalue_z_2))) (struct) (5.0 5.0 5.0)) "Undefined" "OverrideRootScale" null null))

(fn `UserConstructionScript`)