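; Drivable physics car pawn with throttle, steering, mouse look and a handbrake.
; While a rear suspension is in contact, MoveForward pushes the body and adds speed-scaled yaw torque, flipped when reversing, and re-centers unsteered front wheels.
; Steering input sets front wheel yaw through a clamped CalculateWheelZRotation, whose graph holds only an unused expression.
; Tick applies a velocity-scaled force against the body's forward vector while the handbrake is pressed.
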(event `InputAxis|MoveRight`
  (params (AxisValue :type "Float (single-precision)"))
  (set `self.SteerDirection` AxisValue)
  (`SceneComponent.K2_SetRelativeRotation` (`self.Wheel_FR`) (`KismetMathLibrary.MakeRotator` 0.0 0.0 (`KismetMathLibrary.ClampAngle` (`self.CalculateWheelZRotation` (`self.Wheel_FR`) (`self.SteerDirection`)) -60.0 60.0)) false true)
  (`SceneComponent.K2_SetRelativeRotation` (`self.Wheel_FL`) (`KismetMathLibrary.MakeRotator` 0.0 0.0 (`KismetMathLibrary.ClampAngle` (`self.CalculateWheelZRotation` (`self.Wheel_FL`) (`self.SteerDirection`)) -60.0 60.0)) false true))

(event `InputAction|UseWeapon1`
  (params (Key :type "Key Structure")))

(event `InputAxisKey|MouseX`
  (params (AxisValue :type "Float (single-precision)"))
  (bind (_returnvalue_roll _returnvalue_pitch _returnvalue_yaw) (`KismetMathLibrary.BreakRotator` (`self.GetControlRotation`)))
  (`self.AddControllerYawInput` AxisValue)
  (`Controller.SetControlRotation` (`MyBlueprintUtilities.GetLocalPlayerController`) (`KismetMathLibrary.MakeRotator` 0.0 _returnvalue_pitch _returnvalue_yaw)))

(event `InputAxis|MoveForward`
  (params (AxisValue :type "Float (single-precision)"))
  (`self.MoveForward` AxisValue))

(event `InputAxisKey|MouseY`
  (params (AxisValue :type "Float (single-precision)"))
  (`self.AddControllerPitchInput` (* -1 AxisValue)))

(event `MoveForward`
  (params (Direction :type "Float (double-precision)"))
  (bind _steerdirection (`self.SteerDirection`))
  (bind (_relativerotation_roll _relativerotation_pitch _relativerotation_yaw) (`KismetMathLibrary.BreakRotator` (`SceneComponent.RelativeRotation` (`self.Wheel_FL`))))
  (bind (_relativerotation_roll_2 _relativerotation_pitch_2 _relativerotation_yaw_2) (`KismetMathLibrary.BreakRotator` (`SceneComponent.RelativeRotation` (`self.Wheel_FR`))))
  (if (or (`/Game/Vehicles/Cars/Suspension.InContact` (`self.Suspension_RR`)) (`/Game/Vehicles/Cars/Suspension.InContact` (`self.Suspension_RL`)))
    (`PrimitiveComponent.AddForce` (`self.Body`) (* (* (`SceneComponent.GetForwardVector` (`self.Body`)) (`self.Speed`)) Direction) "None" true)
    (`PrimitiveComponent.AddTorqueInRadians` (`self.Body`) (`KismetMathLibrary.MakeVector` 0.0 0.0 (`KismetMathLibrary.Lerp` 0.0 (* (`KismetMathLibrary.SelectFloat` _steerdirection (* _steerdirection -1.0) (>= (`KismetMathLibrary.Dot_VectorVector` (`KismetMathLibrary.Normal` (`self.GetActorForwardVector`)) (`KismetMathLibrary.Normal` (`SceneComponent.GetComponentVelocity` (`self.Body`)))) 0.0)) (`self.TurnSpeed`)) (`KismetMathLibrary.MultiplyMultiply_FloatFloat` (`KismetMathLibrary.FClamp` (`KismetMathLibrary.NormalizeToRange` (`KismetMathLibrary.VSize` (`self.GetVelocity`)) 0.0 500.0)) 3.0))) "None" true)
    (if (== (`self.SteerDirection`) 0.0)
      (`SceneComponent.K2_SetRelativeRotation` (`self.Wheel_FR`) (`KismetMathLibrary.MakeRotator` 0.0 0.0 (`KismetMathLibrary.FInterpTo` _relativerotation_yaw_2 0.0 (`GameplayStatics.GetWorldDeltaSeconds`) 20.0)) false false)
      (`SceneComponent.K2_SetRelativeRotation` (`self.Wheel_FL`) (`KismetMathLibrary.MakeRotator` 0.0 0.0 (`KismetMathLibrary.FInterpTo` _relativerotation_yaw 0.0 (`GameplayStatics.GetWorldDeltaSeconds`) 20.0)) false false))))

(event `self.ReceiveTick`
  (params (DeltaSeconds :type "Float (single-precision)"))
  (if (`self.HandBreakPressed`)
    (`PrimitiveComponent.AddForce` (`self.Body`) (* (`KismetMathLibrary.NegateVector` (`SceneComponent.GetForwardVector` (`self.Body`))) (* (`KismetMathLibrary.FInterpTo` 0.0 (`KismetMathLibrary.VSize` (`SceneComponent.GetComponentVelocity` (`self.Body`))) (`GameplayStatics.GetWorldDeltaSeconds`) 3.0) 1000.0)) "None" true)))

(fn `UserConstructionScript`)